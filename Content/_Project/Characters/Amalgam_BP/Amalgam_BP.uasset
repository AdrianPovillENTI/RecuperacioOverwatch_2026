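; Amalgam is a playable character Blueprint that adds double jump, ape jump and dash skills to its parent character, along with secondary weapon fire.
; BeginPlay initializes health, armor and shield, then registers each skill component, scaling double-jump force from the movement jump velocity.
; Input events fire skills subject to State checks, with dash following camera forward.
; Tick feeds the SpawnPoint transform to the current AmalgamWeapon_BPC.
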(event Input|EnhancedActionEvents|EnhancedInputActionJump
  (params (ActionValue :type Boolean) (ElapsedSeconds :type Float%20%28double-precision%29) (TriggeredSeconds :type Float%20%28double-precision%29) (InputAction :type Input%20Action%20Object%20Reference :default "/Game/_Project/CommonSystems/Input/Jump.Jump"))
  (:Started
    (if (Math|Boolean|ANDBoolean (AI|Components|NavMovement|IsFalling (Variables|Character|GetCharacterMovement self)) (Utilities|Enum|NotEqual(Enum) (Variables|Default|GetState) "NewEnumerator2") (Utilities|Enum|NotEqual(Enum) (Variables|Default|GetState) "NewEnumerator3"))
      (Default|Fire (Variables|Default|GetDoubleJump_BPC)))))

(event Input|EnhancedActionEvents|EnhancedInputActionSkill_0
  (params (ActionValue :type Boolean) (ElapsedSeconds :type Float%20%28double-precision%29) (TriggeredSeconds :type Float%20%28double-precision%29) (InputAction :type Input%20Action%20Object%20Reference :default "/Game/_Project/CommonSystems/Input/Skill_0.Skill_0"))
  (bind _dash_bpc (Variables|Default|GetDash_BPC))
  (:Started
    (if (and (Utilities|Enum|NotEqual(Enum) (Variables|Default|Getstate) "NewEnumerator3") (Utilities|Enum|NotEqual(Enum) (Variables|Default|Getstate) "NewEnumerator2"))
      (Variables|/Game/_Project/Characters/Amalgam_BP/Dash_BPC.Dash_BPC_C|SetDashDir _dash_bpc (Math|Vector|GetForwardVector (Variables|Default|GetCamera)))
      (Default|Fire _dash_bpc))))

(event Input|EnhancedActionEvents|EnhancedInputActionSecondaryFire
  (params (ActionValue :type Boolean) (ElapsedSeconds :type Float%20%28double-precision%29) (TriggeredSeconds :type Float%20%28double-precision%29) (InputAction :type Input%20Action%20Object%20Reference :default "/Game/_Project/CommonSystems/Input/SecondaryFire.SecondaryFire"))
  (bind _weapons (Variables|Default|GetWeapons))
  (bind _currentweaponindex (Variables|Default|GetCurrentWeaponIndex))
  (bind _output (Utilities|Array|Get(acopy) _weapons _currentweaponindex))
  (bind _asamalgam_weapon_bpc (Utilities|Casting|CastToAmalgamWeapon_BPC _output))
  (:Triggered
    (Default|StartSecondFireWeapon _asamalgam_weapon_bpc :!label _label))
  (:Started
    (goto _label))
  (:Canceled
    (Default|StopSecondFireWeapon _asamalgam_weapon_bpc :!label _label_2))
  (:Completed
    (goto _label_2)))

(event Input|EnhancedActionEvents|EnhancedInputActionSkill_1
  (params (ActionValue :type Boolean) (ElapsedSeconds :type Float%20%28double-precision%29) (TriggeredSeconds :type Float%20%28double-precision%29) (InputAction :type Input%20Action%20Object%20Reference :default "/Game/_Project/CommonSystems/Input/Skill_1.Skill_1"))
  (:Triggered
    (if (Utilities|Enum|NotEqual(Enum) (Variables|Default|Getstate) "NewEnumerator3") :!label _label
      (Default|Fire (Variables|Default|GetApeJump_BPC))))
  (:Started
    (goto _label)))

(event EventBeginPlay
  (bind _apejump_bpc (Variables|Default|GetApeJump_BPC))
  (bind _doublejump_bpc (Variables|Default|GetDoubleJump_BPC))
  (bind _dash_bpc (Variables|Default|GetDash_BPC))
  (|CallParentFunction)
  (Utilities|FlowControl|Sequence
    (:then_0
      (CallFunction|InitializeHealth (Utilities|Struct|MakeHealthData 125.0 125.0 5e+01 5e+01 5e+01 5e+01 0.0 false)))
    (:then_1
      (Default|Initialize _doublejump_bpc self "SPACE")
      (Utilities|Array|Add (Variables|Default|GetSkills) _doublejump_bpc)
      (Variables|/Game/_Project/Characters/Amalgam_BP/DoubleJump_BPC.DoubleJump_BPC_C|SetJumpForce _doublejump_bpc (* (Variables|/Script/Engine.CharacterMovementComponent|GetJumpZVelocity (Variables|Character|GetCharacterMovement)) 0.5)))
    (:then_2
      (Default|Initialize _apejump_bpc self "E")
      (Utilities|Array|Add (Variables|Default|GetSkills) _apejump_bpc))
    (:then_3
      (Default|Initialize _dash_bpc self "L SHIFT")
      (Utilities|Array|Add (Variables|Default|GetSkills) _dash_bpc))))

(event Collision|EventActorBeginOverlap
  (params (OtherActor :type Actor%20Object%20Reference)))

(event EventTick
  (params (DeltaSeconds :type Float%20%28single-precision%29))
  (|CallParentFunction DeltaSeconds)
  (Variables|/Game/_Project/Characters/Amalgam_BP/AmalgamWeapon_BPC.AmalgamWeapon_BPC_C|SetSpawnPoint (.AsAmalgam%20Weapon%20BPC (Utilities|Casting|CastToAmalgamWeapon_BPC (Utilities|Array|Get(acopy) (Variables|Default|GetWeapons) (Variables|Default|GetCurrentWeaponIndex)))) (Transformation|GetWorldTransform (Variables|Default|GetSpawnPoint))))

(fn ConstructionScript
  (|CallParentFunction))