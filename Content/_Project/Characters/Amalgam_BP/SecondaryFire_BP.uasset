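; Explosive projectile, apparently the Amalgam character's secondary fire, that deals area damage where it comes to a stop.
; When ProjectileMovement stops, it spawns a scaled-up explosion particle and runs a sphere overlap for Pawns within ExplosionRadius.
; Each pawn with a HealthSystem component takes the full Damage as a non-headshot, with no falloff or instigator filtering, then the projectile destroys itself.
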(event OnProjectileStop(ProjectileMovement)
  (params (ImpactResult :type Hit%20Result%20Structure%20%28by%20ref%29))
  (Effects|SpawnEmitteratLocation "/Game/_Project/StarterContent/Particles/P_Explosion.P_Explosion" (Transformation|GetActorLocation) "0, 0, 0" "5.000000,5.000000,5.000000")
  (bind _outactors (Collision|SphereOverlapActors (Transformation|GetActorLocation) (Variables|Default|GetExplosionRadius) (Utilities|Array|MakeArray "ObjectTypeQuery3") 0))
  (for _array_element _outactors
    (if (Utilities|IsValid (Actor|GetComponentbyClass _array_element "/Game/_Project/CommonSystems/HealthSystem/HealthSystem.HealthSystem_C"))
      (Default|TakeDamage (Actor|GetComponentbyClass _array_element "/Game/_Project/CommonSystems/HealthSystem/HealthSystem.HealthSystem_C") false (Variables|Default|GetDamage))))
  (Actor|DestroyActor))

(event EventBeginPlay)

(event Collision|EventActorBeginOverlap
  (params (OtherActor :type Actor%20Object%20Reference)))

(event EventTick
  (params (DeltaSeconds :type Float%20%28single-precision%29)))

(fn ConstructionScript)